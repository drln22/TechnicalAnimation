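; Anim notify state for a roll after a jump that drives the player character forward using an animation curve.
; Begin resets the stored curve value and disables the player's movement and attack; end re-enables both.
; Each tick teleports the character, without sweep, along capsule forward by the positive change in the "root_translation_Y" curve, acting as manual root motion.
; It always targets player pawn 0, not the animated mesh's owner.
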(fn `Received_NotifyBegin`
  (params (MeshComp :type "SkeletalMeshComponent Object Reference") (Animation :type "AnimSequenceBase Object Reference") (TotalDuration :type "Float (single-precision)") (EventReference :type "AnimNotifyEventReference Structure (by ref)"))
  (returns (ReturnValue :type Boolean))
  (bind _asbp_character (cast `/Game/Character/BP_Character` (`GameplayStatics.GetPlayerPawn` MeshComp)))
  (set `/Game/Character/BP_Character.LastCurveValue` 0.0 _asbp_character)
  (set `/Game/Character/BP_Character.canMove` false _asbp_character)
  (set `/Game/Character/BP_Character.canAttack` false _asbp_character)
  (return false))

(fn `Received_NotifyEnd`
  (params (MeshComp :type "SkeletalMeshComponent Object Reference") (Animation :type "AnimSequenceBase Object Reference") (EventReference :type "AnimNotifyEventReference Structure (by ref)"))
  (returns (ReturnValue :type Boolean))
  (bind _asbp_character (cast `/Game/Character/BP_Character` (`GameplayStatics.GetPlayerPawn` MeshComp)))
  (set `/Game/Character/BP_Character.canMove` true _asbp_character)
  (set `/Game/Character/BP_Character.canAttack` true _asbp_character)
  (return false))

(fn `Received_NotifyTick`
  (params (MeshComp :type "SkeletalMeshComponent Object Reference") (Animation :type "AnimSequenceBase Object Reference") (FrameDeltaTime :type "Float (single-precision)") (EventReference :type "AnimNotifyEventReference Structure (by ref)"))
  (returns (ReturnValue :type Boolean))
  (bind _returnvalue (`AnimInstance.GetCurveValue` (`SkeletalMeshComponent.GetAnimInstance` MeshComp) "root_translation_Y"))
  (bind _asbp_character (cast `/Game/Character/BP_Character` (`GameplayStatics.GetPlayerPawn` MeshComp)))
  (bind _returnvalue_2 (`KismetMathLibrary.MakeVector` (- _returnvalue (`/Game/Character/BP_Character.LastCurveValue` _asbp_character))))
  (`Actor.K2_SetActorLocation` _asbp_character (+ (`SceneComponent.K2_GetComponentLocation` (`Actor.RootComponent` _asbp_character)) (`KismetMathLibrary.GreaterGreater_VectorRotator` (select `bool` (<= (.x _returnvalue_2) 0.0) :`false` _returnvalue_2) (`SceneComponent.K2_GetComponentRotation` (`Character.CapsuleComponent` _asbp_character)))) false true)
  (set `/Game/Character/BP_Character.LastCurveValue` _returnvalue _asbp_character)
  (return false))