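; BP_Enemy is a melee enemy character that chases the player and dies when its health runs out.
; PawnSensing triggers an AI move toward the player, and reaching acceptance range starts a CanAttack-gated, delay-timed montage call and box trace that applies damage.
; Tick halts movement while the player is unseen, though the seen flag is never cleared once set.
; Debug prints and persistent trace drawing remain, and the montage call has no animation assigned.
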(event `self.ReceiveAnyDamage`
  (params (Damage :type "Float (single-precision)") (DamageType :type "DamageType Object Reference") (InstigatedBy :type "Controller Object Reference") (DamageCauser :type "Actor Object Reference"))
  ;[0.15 0 0.006926 0.5] Take Damage
  (set `self.Health` (- (`self.Health`) Damage))
  (if (> (`self.Health`) 0.0)
    (`KismetSystemLibrary.PrintString` "damage")
    (else
      (`self.K2_DestroyActor`))))

(event `self.PawnSensing.OnSeePawn`
  (params (Pawn :type "Pawn Object Reference"))
  ;[0 0.1291 0.15 0.5] Enemy AI (manca l'animazione)
  (set `self.isSeeingPlayer` true)
  (`self.FollowPlayer`))

(event `FollowPlayer`
  ;[0 0.1291 0.15 0.5] Enemy AI (manca l'animazione)
  (if (`self.isSeeingPlayer`)
    (`|AIMoveTo` self (0.0 0.0 0.0) (`GameplayStatics.GetPlayerCharacter` 0) 350.0
      (:`OnSuccess`
        (if (`self.canAttack`)
          (set `self.canAttack` false)
          (`self.PlayAnimMontage` null)
          (`KismetSystemLibrary.Delay` 0.4)
          (bind _outhit (`KismetSystemLibrary.BoxTraceSingle` :`Start` (`SceneComponent.GetSocketLocation` (`self.StartAttack`) "None") :`End` (`SceneComponent.GetSocketLocation` (`self.EndAttack`) "None") :`HalfSize` (220.0 220.0 40.0) :`TraceChannel` "TraceTypeQuery1" :`DrawDebugType` "Persistent"))
          (`GameplayStatics.ApplyDamage` (`.HitActor` (`GameplayStatics.BreakHitResult` _outhit)) 50.0)
          (`KismetSystemLibrary.PrintString` "damaged player")
          (`KismetSystemLibrary.Delay` 0.6)
          (set `self.canAttack` true))))
    (else
      (set `self.isSeeingPlayer` false))))

(event `self.ReceiveTick`
  (params (DeltaSeconds :type "Float (single-precision)"))
  ;[0 0.1291 0.15 0.5] Enemy AI (manca l'animazione)
  (if (not (`self.isSeeingPlayer`))
    (`MovementComponent.StopMovementImmediately` (`self.CharacterMovement`))))

(fn `UserConstructionScript`)