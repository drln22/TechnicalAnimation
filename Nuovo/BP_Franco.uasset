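; Boss character Franco: plays an intro montage, attaches a hammer to its hand, shows a health bar, and ragdolls from its death montage.
; Tick keeps it facing the player and refreshes the health bar.
; Attack, not called within this graph, picks by distance among leap, dash sweep, hammer sweeps, kick or a strafing pause, with some randomness.
; Montage notifies trigger launches toward the player and debug-drawn box traces that apply damage.
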(event `Event Attacca_martello_alla_mano`
  ;[0 0.07971 0.15 0.5] Brandisci Martello
  (bind _returnvalue (`|SpawnActorFromClass` "/Game/Enemy/Nuovo/Franco_arma/BP_Franco_martello.BP_Franco_martello_C" (`SceneComponent.GetSocketTransform` (`self.Mesh`) "D_manoSocket" "RTS_World") "Undefined" "MultiplyWithRoot" null null))
  (`self.K2_AttachToComponent` _returnvalue (`self.Mesh`) "D_manoSocket" "SnapToTarget" "SnapToTarget" "SnapToTarget" true))

(event `self.ReceiveBeginPlay`
  ; Begin play e event Tick
  (`self.Widget vita`)
  (`self.Animazione iniziale`)
  (`KismetSystemLibrary.Delay` 8.0)
  (`self.Event Attacca_martello_alla_mano`))

(event `self.ReceiveAnyDamage`
  (params (Damage :type "Float (single-precision)") (DamageType :type "DamageType Object Reference") (InstigatedBy :type "Controller Object Reference") (DamageCauser :type "Actor Object Reference"))
  ;[0.1466 0.15 0 0.5] Prendi danno
  (if (not (`self.è gia morto`))
    (set `self.VitaFranco` (- (`self.VitaFranco`) Damage))
    (if (<= (`self.VitaFranco`) 0.0)
      (`CharacterMovementComponent.SetMovementMode` (`self.CharacterMovement`) "MOVE_None" 0)
      (`|PlayMontage` (`self.Mesh`) "/Game/Enemy/Nuovo/Franco_Animations/Franco_morte_Montage.Franco_morte_Montage"
        (:`OnNotifyBegin`
          (`PrimitiveComponent.SetSimulatePhysics` (`self.Mesh`) true))))))

(event `self.ReceiveTick`
  (params (DeltaSeconds :type "Float (single-precision)"))
  ; Begin play e event Tick
  (`self.Guarda sempre il giocatore`)
  (`self.Vita residua`))

(event `Animazione iniziale`
  (bind _returnvalue (`SkeletalMeshComponent.GetAnimInstance` (`self.Mesh`)))
  ;[0.15 0.1422 0 0.5] Animazione iniziale
  (set `self.Inizio Scontro` true)
  (`CharacterMovementComponent.SetMovementMode` (`self.CharacterMovement`) "MOVE_None" 0)
  (`|PlayMontage` (`self.Mesh`) "/Game/Enemy/Nuovo/Franco_Animations/Franco_Inizio_scontro_Montage.Franco_Inizio_scontro_Montage"
    (:`OnNotifyBegin`
      (`AnimInstance.Montage_Pause` _returnvalue "/Game/Enemy/Nuovo/Franco_Animations/Franco_Inizio_scontro_Montage.Franco_Inizio_scontro_Montage")
      (`KismetSystemLibrary.Delay` 3.0)
      (`AnimInstance.Montage_Resume` _returnvalue "/Game/Enemy/Nuovo/Franco_Animations/Franco_Inizio_scontro_Montage.Franco_Inizio_scontro_Montage")
      (`KismetSystemLibrary.Delay` 4.0)
      (set `self.Inizio Scontro` false)
      (`CharacterMovementComponent.SetMovementMode` (`self.CharacterMovement`) "MOVE_Walking" 0)
      (set `self.VitaFranco` 500.0))))

(event `Widget vita`
  ;[0 0.15 0.07238 0.5] Widget vita
  (bind _returnvalue (`|CreateWidget` "/Game/Enemy/Nuovo/Franco_UI/HPFranco.HPFranco_C"))
  (`UserWidget.AddToViewport` _returnvalue 0)
  (set `self.VitaFranco_UI` _returnvalue))

(event `Aspetta`
  ;[0.15 0.1196 0 0.5] Aspetta e dai tregua al giocatore
  (if (not (`self.isAttacking`))
    (`|PlayMontage` (`self.Mesh`) "/Game/Enemy/Nuovo/Franco_Animations/Franco_cammina_a_sinistra_Montage.Franco_cammina_a_sinistra_Montage"
      (:`then`
        (set `self.isAttacking` true))
      (:`OnCompleted`
        (set `self.isAttacking` false)))))

(event `Guarda sempre il giocatore`
  (bind (_returnvalue_roll _returnvalue_pitch) (`KismetMathLibrary.BreakRotator` (`self.K2_GetActorRotation`)))
  (bind (_returnvalue_roll_2 _returnvalue_pitch_2 _returnvalue_yaw) (`KismetMathLibrary.BreakRotator` (`KismetMathLibrary.FindLookAtRotation` (`self.K2_GetActorLocation`) (`self.K2_GetActorLocation` (`GameplayStatics.GetPlayerCharacter` 0)))))
  ;[0.1203 0.03398 0.15 0.5] Guarda costantemente il giocatore
  (`self.K2_SetActorRotation` (`KismetMathLibrary.MakeRotator` _returnvalue_roll _returnvalue_pitch _returnvalue_yaw)))

(event `Vita residua`
  ;[0 0.15 0.07238 0.5] Widget vita
  (`ProgressBar.SetPercent` (`/Game/Enemy/Nuovo/Franco_UI/HPFranco.VitaFrancoBar` (`self.VitaFranco_UI`)) (/ (`self.VitaFranco`) 500.0)))

(event `Scatto salto`
  (bind _returnvalue (- (`self.K2_GetActorLocation` (`GameplayStatics.GetPlayerCharacter` 0)) (`self.K2_GetActorLocation`)))
  ;[0.1368 0.0263 0.15 0.5] Scatto Salto
  (if (`self.Scatto`)
    (`self.LaunchCharacter` (* (`KismetMathLibrary.Normal` _returnvalue) (/ (`KismetMathLibrary.VSize` _returnvalue) 0.03)) true true)
    (set `self.Scatto` false)
    (else
      (set `self.Scatto` false))))

(event `/Game/Enemy/Nuovo/Franco_AI/BPI_BossFight.Attack`
  ;[0.09969 0.01887 0.15 0.5] Scegli tipo di attacco in base alla distanza
  (set `self.DistanzaMassimaAttacco` (`KismetMathLibrary.VSize` (- (`self.K2_GetActorLocation`) (`self.K2_GetActorLocation` (`GameplayStatics.GetPlayerCharacter` 0)))))
  (if (`self.Inizio Scontro`)
    _
    (elif (>= (`self.DistanzaMassimaAttacco`) 1400.0)
      (set `self.Scatto` true)
      (`self.Event attacco in salto`)
      (elif (>= (`self.DistanzaMassimaAttacco`) 700.0)
        (switch `int` (`KismetMathLibrary.RandomInteger` 4)
          (:`0`
            (set `self.Distanza scatto ravvicinato` true :!label _label)
            (`self.ScattoSpazzata`))
          (:`1`
            (goto _label))
          (:`2`
            (goto _label))
          (:`3`
            (`self.Aspetta`)))
        (elif (>= (`self.DistanzaMassimaAttacco`) 350.0)
          (`KismetSystemLibrary.Delay` 0.8)
          (switch `int` (`KismetMathLibrary.RandomInteger` 5)
            (:`0`
              (`self.Event Spazzata`))
            (:`1`
              (`self.Spazzata al contrario`))
            (:`2`
              (`self.Aspetta` :!label _label_2))
            (:`3`
              (goto _label_2)))
          (else
            (`KismetSystemLibrary.Delay` 0.8)
            (`self.Event calcio`)))))))

(event `Event attacco in salto`
  (bind _endattack (`self.EndAttack`))
  (bind _returnvalue (`SceneComponent.K2_GetComponentLocation` _endattack))
  ;[0.15 0.05353 0 0.5] Box danno attacco in salto
  ;;[0.15 0.02277 0.01986 0.5] Attacco in salto
  (if (not (`self.isAttacking`))
    (bind _notifyname (`|PlayMontage` (`self.Mesh`) "/Game/Enemy/Nuovo/Franco_Animations/Franco_attacco_in_salto_daFermo_Montage.Franco_attacco_in_salto_daFermo_Montage")
      (:`then`
        (set `self.isAttacking` true))
      (:`OnCompleted`
        (set `self.isAttacking` false))
      (:`OnNotifyBegin`
        (switch `string` (`KismetStringLibrary.Conv_NameToString` _notifyname)
          (:`uno`
            (`self.Scatto salto`))
          (:`due`
            (bind (_outhit _returnvalue_2) (`KismetSystemLibrary.BoxTraceSingleForObjects` :`Start` _returnvalue :`End` (+ _returnvalue (* (`KismetMathLibrary.GetForwardVector` (`SceneComponent.K2_GetComponentRotation` _endattack)) 200.0)) :`HalfSize` (250.0 100.0 50.0) :`ObjectTypes` (`|MakeArray` "ObjectTypeQuery1" :!type "EObjectTypeQuery Enum") :`DrawDebugType` "ForDuration" :`DrawTime` 2.0))
            (if _returnvalue_2
              (`GameplayStatics.ApplyDamage` (`.HitActor` (`GameplayStatics.BreakHitResult` _outhit)) 50.0))))))))

(event `Event Spazzata`
  (bind _endattack (`self.EndAttack`))
  (bind _returnvalue (`SceneComponent.K2_GetComponentLocation` _endattack))
  ;[0.15 0.05353 0 0.5] Box danno martellata
  ;;[0.15 0.02277 0.01986 0.5] Martellata
  (if (not (`self.isAttacking`))
    (`|PlayMontage` (`self.Mesh`) "/Game/Enemy/Nuovo/Franco_Animations/Franco_spazzata_Montage.Franco_spazzata_Montage"
      (:`then`
        (set `self.isAttacking` true))
      (:`OnCompleted`
        (set `self.isAttacking` false))
      (:`OnNotifyBegin`
        (bind (_outhit _returnvalue_2) (`KismetSystemLibrary.BoxTraceSingleForObjects` :`Start` _returnvalue :`End` (+ _returnvalue (* (`KismetMathLibrary.GetForwardVector` (`SceneComponent.K2_GetComponentRotation` _endattack)) 200.0)) :`HalfSize` (200.0 150.0 50.0) :`ObjectTypes` (`|MakeArray` "ObjectTypeQuery1" :!type "EObjectTypeQuery Enum") :`DrawDebugType` "ForDuration" :`DrawTime` 2.0))
        (if _returnvalue_2
          (`GameplayStatics.ApplyDamage` (`.HitActor` (`GameplayStatics.BreakHitResult` _outhit)) 20.0))))))

(event `Scatto corsa`
  (bind _returnvalue (- (`self.K2_GetActorLocation` (`GameplayStatics.GetPlayerCharacter` 0)) (`self.K2_GetActorLocation`)))
  ;[0.1368 0.0263 0.15 0.5] Scatto corsa
  (if (`self.Distanza scatto ravvicinato`)
    (`self.LaunchCharacter` (* (`KismetMathLibrary.Normal` _returnvalue) (/ (`KismetMathLibrary.VSize` _returnvalue) 0.05)) true true)
    (set `self.Distanza scatto ravvicinato` false)
    (else
      (set `self.Distanza scatto ravvicinato` false))))

(event `ScattoSpazzata`
  (bind _startattack (`self.StartAttack`))
  (bind _returnvalue (`SceneComponent.K2_GetComponentLocation` _startattack))
  ;[0.15 0.05353 0 0.5] Box danno scatto spazzata
  ;;[0.15 0.02277 0.01986 0.5] scatto spazzata
  (if (not (`self.isAttacking`))
    (bind _notifyname (`|PlayMontage` (`self.Mesh`) "/Game/Enemy/Nuovo/Franco_Animations/Franco_scatto_spazzata_Montage.Franco_scatto_spazzata_Montage")
      (:`then`
        (set `self.isAttacking` true))
      (:`OnCompleted`
        (set `self.isAttacking` false))
      (:`OnNotifyBegin`
        (switch `string` (`KismetStringLibrary.Conv_NameToString` _notifyname)
          (:`uno`
            (`self.Scatto corsa`))
          (:`due`
            (bind (_outhit _returnvalue_2) (`KismetSystemLibrary.BoxTraceSingleForObjects` :`Start` _returnvalue :`End` (+ _returnvalue (* (`KismetMathLibrary.GetForwardVector` (`SceneComponent.K2_GetComponentRotation` _startattack)) 200.0)) :`HalfSize` (200.0 150.0 50.0) :`ObjectTypes` (`|MakeArray` "ObjectTypeQuery1" :!type "EObjectTypeQuery Enum") :`DrawDebugType` "ForDuration" :`DrawTime` 2.0))
            (if _returnvalue_2
              (`GameplayStatics.ApplyDamage` (`.HitActor` (`GameplayStatics.BreakHitResult` _outhit)) 30.0))))))))

(event `Spazzata al contrario`
  (bind _endattack (`self.EndAttack`))
  (bind _returnvalue (`SceneComponent.K2_GetComponentLocation` _endattack))
  ;[0.15 0.05353 0 0.5] Box danno martellata al contrario
  ;;[0.15 0.02277 0.01986 0.5] Martellata al contrario
  (if (not (`self.isAttacking`))
    (`|PlayMontage` (`self.Mesh`) "/Game/Enemy/Nuovo/Franco_Animations/Franco_spazzata_Montage2.Franco_spazzata_Montage2"
      (:`then`
        (set `self.isAttacking` true))
      (:`OnCompleted`
        (set `self.isAttacking` false))
      (:`OnNotifyBegin`
        (bind (_outhit _returnvalue_2) (`KismetSystemLibrary.BoxTraceSingleForObjects` :`Start` _returnvalue :`End` (+ _returnvalue (* (`KismetMathLibrary.GetForwardVector` (`SceneComponent.K2_GetComponentRotation` _endattack)) 200.0)) :`HalfSize` (200.0 150.0 50.0) :`ObjectTypes` (`|MakeArray` "ObjectTypeQuery1" :!type "EObjectTypeQuery Enum") :`DrawDebugType` "ForDuration" :`DrawTime` 2.0))
        (if _returnvalue_2
          (`GameplayStatics.ApplyDamage` (`.HitActor` (`GameplayStatics.BreakHitResult` _outhit)) 20.0))))))

(event `Event calcio`
  (bind _startattack (`self.StartAttack`))
  (bind _returnvalue (`SceneComponent.K2_GetComponentLocation` _startattack))
  ;[0.15 0.05353 0 0.5] Box danno calcio
  ;;[0.15 0.02277 0.01986 0.5] Calcio
  (if (not (`self.isAttacking`))
    (`|PlayMontage` (`self.Mesh`) "/Game/Enemy/Nuovo/Franco_Animations/Franco_calcio_Montage.Franco_calcio_Montage"
      (:`then`
        (set `self.isAttacking` true))
      (:`OnCompleted`
        (set `self.isAttacking` false))
      (:`OnNotifyBegin`
        (bind (_outhit _returnvalue_2) (`KismetSystemLibrary.BoxTraceSingleForObjects` :`Start` _returnvalue :`End` (+ _returnvalue (* (`KismetMathLibrary.GetForwardVector` (`SceneComponent.K2_GetComponentRotation` _startattack)) 200.0)) :`HalfSize` (30.0 40.0 50.0) :`ObjectTypes` (`|MakeArray` "ObjectTypeQuery1" :!type "EObjectTypeQuery Enum") :`DrawDebugType` "ForDuration" :`DrawTime` 2.0))
        (if _returnvalue_2
          (`GameplayStatics.ApplyDamage` (`.HitActor` (`GameplayStatics.BreakHitResult` _outhit)) 30.0))))))

(fn `UserConstructionScript`)